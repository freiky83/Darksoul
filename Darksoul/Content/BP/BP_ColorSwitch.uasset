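; Blueprint actor that animates the color of its cube mesh back and forth each time SwitchColor is triggered.
; The construction script creates a dynamic instance of MI_BaseColor, stores it as BodyPaint and applies it to the cube.
; A FlipFlop alternately plays and reverses ColorSwitchTimeline, whose color track drives the BaseColor parameter.
; Debug prints show an accumulated timer, reset when the timeline finishes.
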(event `SwitchColor`
  (`/Engine/EditorBlueprintResources/StandardMacros.FlipFlop`
    (:`A`
      (bind (_direction _matcolor) (`Timeline|ColorSwitchTimeline` :!via `PlayFromStart` :!label _label)
        (:`Update`
          (`MaterialInstanceDynamic.SetVectorParameterValue` (`self.BodyPaint`) "BaseColor" _matcolor)
          ;[1 1 1] Debug (Display Timer and when finished)
          (bind _output_get (set `self.timer` (+ (`GameplayStatics.GetWorldDeltaSeconds`) (`self.timer`))))
          (`KismetSystemLibrary.PrintString` (`KismetStringLibrary.Conv_DoubleToString` _output_get)))
        (:`Finished`
          (`KismetSystemLibrary.PrintString` "Finished")
          (set `self.timer` 0.0))))
    (:`B`
      (goto _label :!via `ReverseFromEnd`))))

(fn `UserConstructionScript`
  (bind _returnvalue (`KismetMaterialLibrary.CreateDynamicMaterialInstance` "/Game/Materials/MI_BaseColor.MI_BaseColor"))
  (bind _output_get (set `self.BodyPaint` _returnvalue))
  (`PrimitiveComponent.SetMaterial` (`self.Cube`) 0 _output_get))